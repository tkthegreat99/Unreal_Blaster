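; GM_OurGame is a game mode that tracks collectibles left to gather and opens the gate when none remain.
; RegisterCollectible raises the count and CollectibleCollected lowers it, refreshing the player UI and checking for zero.
; At zero it finds the BP_Gate actor by class and calls OpenDoor.
; BeginPlay waits briefly before the first UI update.
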(event Custom|RegisterCollectible
  (Math|Integer|IncrementInt (Variables|Default|GetNumItemsToCollect)))

(event Custom|CollectibleCollected
  (Math|Integer|DecrementInt (Variables|Default|GetNumItemsToCollect)
    (:%20%20
      (CallFunction|UpdateCollectibleUI)
      (bind _alldestroyed (CallFunction|CheckforAllCollectiblesDestroyed))
      (if _alldestroyed
        (CallFunction|OpenMasterDoor)))))

(event EventBeginPlay
  (Utilities|FlowControl|Delay 0.2)
  (CallFunction|UpdateCollectibleUI))

(fn ConstructionScript)

(fn CheckforAllCollectiblesDestroyed
  (return (<= (Variables|Default|GetNumItemsToCollect) 0)))

(fn OpenMasterDoor
  (bind _returnvalue (Actor|GetActorOfClass "/Game/BlueprintSaveLoad/Blueprints/BP_Gate.BP_Gate_C"))
  (Default|OpenDoor _returnvalue))

(fn UpdateCollectibleUI
  (Default|SetCollectibleDisplay (Variables|Default|GetPlayerUIRef) (Variables|Default|GetNumItemsToCollect)))